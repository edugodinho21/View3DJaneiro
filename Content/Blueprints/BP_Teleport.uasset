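; BP_Teleport is a teleport point actor that hides itself when a player, identified by the BI_IsPlayer interface, overlaps its box.
; Begin overlap hides the mesh and disables box collision; end overlap restores both after a half-second delay, with debug prints.
; Getter functions expose its clickable flag, name and arrow location as a position, while SwitchVisibility lets callers hide it directly.
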(event `self.Box.OnComponentBeginOverlap`
  (params (OverlappedComponent :type "PrimitiveComponent Object Reference") (OtherActor :type "Actor Object Reference") (OtherComp :type "PrimitiveComponent Object Reference") (OtherBodyIndex :type Integer) (bFromSweep :type Boolean) (SweepResult :type "HitResult Structure (by ref)"))
  (if (`KismetSystemLibrary.DoesImplementInterface` OtherActor "/Game/Blueprints/BI_IsPlayer.BI_IsPlayer_C")
    (`SceneComponent.SetVisibility` (`self.StaticMesh`) false true)
    (`PrimitiveComponent.SetCollisionEnabled` (`self.Box`) "NoCollision")))

(event `self.Box.OnComponentEndOverlap`
  (params (OverlappedComponent :type "PrimitiveComponent Object Reference") (OtherActor :type "Actor Object Reference") (OtherComp :type "PrimitiveComponent Object Reference") (OtherBodyIndex :type Integer))
  (if (`KismetSystemLibrary.DoesImplementInterface` OtherActor "/Game/Blueprints/BI_IsPlayer.BI_IsPlayer_C")
    (`KismetSystemLibrary.PrintString` "END SUCCESS")
    (`KismetSystemLibrary.Delay` 0.5)
    (`SceneComponent.SetVisibility` (`self.StaticMesh`) true true)
    (`PrimitiveComponent.SetCollisionEnabled` (`self.Box`) "QueryOnly")
    (else
      (`KismetSystemLibrary.PrintString` "END FAILED"))))

(fn `Check Clickable`
  (returns (NewParam :type Boolean))
  (return (`self.Clicked`)))

(fn `Check Position`
  (returns (NewParam :type "Vector Structure"))
  (return (`SceneComponent.K2_GetComponentLocation` (`self.Arrow`))))

(fn `Get Name`
  (returns (Name :type Text))
  (return (`self.Name`)))

(fn `Switch Visibility`
  (returns (NewParam :type Boolean))
  (`SceneComponent.SetVisibility` (`self.StaticMesh`) false true)
  (`PrimitiveComponent.SetCollisionEnabled` (`self.Box`) "NoCollision")
  (return true))

(fn `UserConstructionScript`)